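; Gameplay ability that handles a non-hit reaction when the owner's posture breaks.
; On a Combat.Event.PostureBroken event it applies the posture-broken and stun gameplay effects to itself, then calls the parent's activation; other event tags get no handling.
; It overrides ResolveAnimation to supply the NonHitImpact animation from the weapon's animation data.
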(event Ability|EventActivateAbilityFromEvent
  (params (EventData :type Gameplay%20Event%20Data%20Structure%20%28by%20ref%29))
  (bind _returnvalue (Ability|GetAbilitySystemComponentfromActorInfo))
  (if (== (.EventTag (Utilities|Struct|BreakGameplayEventData EventData)) "(TagName=\"Combat.Event.PostureBroken\")")
    (GameplayEffects|ApplyGameplayEffectToSelf :self _returnvalue :GameplayEffectClass "/Game/GAS/GameplayEffects/GE_PostureBroken.GE_PostureBroken_C")
    (GameplayEffects|ApplyGameplayEffectToSelf :self _returnvalue :GameplayEffectClass "/Game/GAS/GameplayEffects/GE_Stun.GE_Stun_C")
    (|CallParentFunction)))

(fn ResolveAnimation
  (return (Variables|/Script/GASAssignment.PDA_WeaponAnimationData|GetNonHitImpact (Variables|/Script/GASAssignment.Weapon|GetWeaponAnimationData (Variables|Default|GetWeapon)))))