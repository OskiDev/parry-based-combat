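; Gameplay ability that draws the owner's weapon from its stowed position into its held socket.
; On activation it gets the weapon through a message to the owner actor, checks its data and commits the ability.
; It plays the weapon's draw montage, whose Grab Weapon notify plays a sound and attaches the weapon using its data's transform and socket.
; The ability ends on montage blend-out or most failed checks, but not when the weapon is invalid.
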(event Ability|EventActivateAbility
  (bind _returnvalue (Ability|GetActorInfo))
  (bind _returnvalue_2 (Ability|GetActorInfo))
  (bind (_owneractor _skeletalmeshcomponent) (Utilities|Struct|BreakGameplayAbilityActorInfo _returnvalue))
  (bind (_owneractor_2 _skeletalmeshcomponent_2) (Utilities|Struct|BreakGameplayAbilityActorInfo _returnvalue_2))
  (Utilities|IsValid _skeletalmeshcomponent
    (:Is%20Valid
      (bind _returnvalue_3 (Class|CombatInterface|GetOwnerWeapon(Message) _owneractor))
      (bind _output_get (Variables|Default|SetOwnerWeapon _returnvalue_3))
      (Utilities|IsValid _output_get
        (:Is%20Valid
          (Utilities|IsValid (Variables|/Script/GASAssignment.Weapon|GetWeaponBaseData _output_get)
            (:Is%20Valid
              (Utilities|IsValid (Variables|/Script/GASAssignment.Weapon|GetWeaponAnimationData _output_get)
                (:Is%20Valid
                  (bind _returnvalue_4 (Ability|CommitAbility))
                  (if _returnvalue_4
                    (bind _notifyname (Animation|Montage|PlayMontage _skeletalmeshcomponent_2 (Variables|/Script/GASAssignment.PDA_WeaponAnimationData|GetDrawWeaponMontage (Variables|/Script/GASAssignment.Weapon|GetWeaponAnimationData (Variables|Default|GetOwnerWeapon))))
                      (:OnBlendOut
                        (Ability|EndAbility))
                      (:OnNotifyBegin
                        (switch name _notifyname
                          (:GrabWeapon
                            (Audio|PlaySoundatLocation "/Game/Sounds/SC_DrawSword.SC_DrawSword" (Transformation|GetActorLocation _owneractor_2) "0, 0, 0" 1.0 1.0 0.0 0 0 0 0)
                            (Transformation|SetActorRelativeTransform (Variables|Default|GetOwnerWeapon) (Variables|/Script/GASAssignment.PDA_WeaponBaseData|GetHeldWeaponTransform (Variables|/Script/GASAssignment.Weapon|GetWeaponBaseData (Variables|Default|GetOwnerWeapon))) false false)
                            (Transformation|AttachComponentToComponent (Variables|Default|GetOwnerWeapon) (Utilities|Struct|BreakGameplayAbilityActorInfo (Ability|GetActorInfo)) (Variables|/Script/GASAssignment.PDA_WeaponBaseData|GetHeldSocket (Variables|/Script/GASAssignment.Weapon|GetWeaponBaseData (Variables|Default|GetOwnerWeapon))) "KeepRelative" "KeepRelative" "KeepRelative" false)))))
                    (else
                      (Ability|EndAbility :!label _label))))
                (:Is%20Not%20Valid
                  (goto _label))))
            (:Is%20Not%20Valid
              (goto _label))))))
    (:Is%20Not%20Valid
      (goto _label))))