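; Base gameplay ability for reactions that plays a montage on the owner's skeletal mesh.
; Activation caches the owner's weapon, gets a montage from ResolveAnimation, commits, then plays it between PreMontageEvent and PostMontageEvent, all three empty stubs for child classes.
; Blend-out, interruption and failed checks share one exit that runs PostMontageEvent, resets the weapon's ignore array and ends the ability.
; Ending the ability stops the montage instantly.
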(event Ability|EventActivateAbility
  (bind _returnvalue (Ability|GetActorInfo))
  (bind (_owneractor _skeletalmeshcomponent) (Utilities|Struct|BreakGameplayAbilityActorInfo _returnvalue))
  (bind _returnvalue_2 (Class|CombatInterface|GetOwnerWeapon(Message) _owneractor))
  (Variables|Default|SetWeapon _returnvalue_2)
  (bind _animation (CallFunction|ResolveAnimation))
  (Utilities|IsValid _animation
    (:Is%20Valid
      (bind _returnvalue_3 (Ability|CommitAbility))
      (if _returnvalue_3
        (CallFunction|PreMontageEvent)
        (Animation|Montage|PlayMontage _skeletalmeshcomponent _animation 1.0 0.0 "None" (Variables|Default|GetShouldStopAllMontages)
          (:OnBlendOut
            _)
          (:OnInterrupted
            _))))
    (:Is%20Not%20Valid
      _))
  (CallFunction|PostMontageEvent)
  (Class|Weapon|ResetIgnoreArray _returnvalue_2)
  (Ability|EndAbility))

(event Ability|EventOnEndAbility
  (params (bWasCancelled :type Boolean))
  (Animation|Montage|MontageStop (Components|SkeletalMesh|GetAnimInstance (.SkeletalMeshComponent (Utilities|Struct|BreakGameplayAbilityActorInfo (Ability|GetActorInfo)))) 0.0 (stale Ability|EventActivateAbility _animation)))

(fn ResolveAnimation
  (return 0))

(fn PreMontageEvent)

(fn PostMontageEvent)