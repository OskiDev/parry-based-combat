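; Melee combo attack gameplay ability for players and AI, playing montages from the owner weapon's combo data.
; Montage notifies open hitbox windows, where a looping timer runs weapon traces, and combo windows, where buffered input or an AI random roll chains the next attack.
; Hit events resolve into damage, block or parry via gameplay effects and cues, with block and parry requiring opposed facing.
; Non-ASC hits and some parries interrupt the combo.
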(event Custom|WaitForComboInput
  (Ability|Tasks|WaitInputPress false
    (:OnPress
      (if (and (GameplayTags|HasMatchingGameplayTag (Ability|GetAbilitySystemComponentfromActorInfo) "(TagName=\"Combat.State.Attacking.ComboActive\")") (not (Variables|Default|GetComboInterrupted)))
        (Variables|Default|SetShouldCombo true))
      (CallFunction|WaitforComboInput))))

(event Custom|TriggerNextCombo
  (bind _returnvalue (Ability|GetOwningActorfromActorInfo))
  (bind _returnvalue_2 (Ability|GetOwningActorfromActorInfo))
  (bind _waithitactortask (Variables|Default|GetWaitHitActorTask))
  (bind _ownerweapon (Variables|Default|GetOwnerWeapon))
  (if (not (Variables|Default|GetComboInterrupted))
    (Variables|Default|SetShouldCombo false)
    (bind _notifyname (Animation|Montage|PlayMontage (Utilities|Struct|BreakGameplayAbilityActorInfo (Ability|GetActorInfo)) (.montage (Utilities|Array|Get(acopy) (Variables|Default|GetAttackMontageArray) (Variables|Default|GetCurrentComboIndex))))
      (:OnBlendOut
        (CallFunction|EndAbility))
      (:OnNotifyBegin
        (switch name _notifyname
          (:HitboxActive
            (Ability|GameplayEffect|AddLooseGameplayTags _returnvalue_2 (GameplayTags|MakeGameplayTagContainerfromTag "(TagName=\"Combat.State.Attacking.HitboxActive\")"))
            (CallFunction|BindHitboxActive)
            (Audio|PlaySoundatLocation "/Game/Sounds/SC_Slash.SC_Slash" (Transformation|GetActorLocation (Utilities|Struct|BreakGameplayAbilityActorInfo (Ability|GetActorInfo))) "0, 0, 0" 1.0 1.0 0.0 0 0 0 0))
          (:ComboWindow
            (Ability|GameplayEffect|AddLooseGameplayTags _returnvalue_2 (GameplayTags|MakeGameplayTagContainerfromTag "(TagName=\"Combat.State.Attacking.ComboActive\")")))))
      (:OnNotifyEnd
        (if (Class|AbilitySystemBlueprintLibrary|IsGameplayAbilityActive)
          (switch name _notifyname
            (:HitboxActive
              (Ability|GameplayEffect|RemoveLooseGameplayTags _returnvalue (GameplayTags|MakeGameplayTagContainerfromTag "(TagName=\"Combat.State.Attacking.HitboxActive\")"))
              (CallFunction|UnbindHitboxActive)
              (Utilities|IsValid _waithitactortask
                (:Is%20Valid
                  (GameplayTasks|EndTask _waithitactortask))
                (:Is%20Not%20Valid
                  _))
              (Utilities|IsValid _ownerweapon
                (:Is%20Valid
                  (Class|Weapon|ResetIgnoreArray _ownerweapon))))
            (:ComboWindow
              (Ability|GameplayEffect|RemoveLooseGameplayTags _returnvalue (GameplayTags|MakeGameplayTagContainerfromTag "(TagName=\"Combat.State.Attacking.ComboActive\")"))
              (if (Variables|Default|GetShouldCombo)
                (bind _result (Math|Integer|IncrementInt (Variables|Default|GetCurrentComboIndex) :!label _label)
                  (:%20%20
                    (if (not (> _result (Utilities|Array|LastIndex (Variables|Default|GetAttackMontageArray))))
                      (CallFunction|TriggerNextCombo))))
                (elif (Variables|Default|GetIsAIControlled)
                  (if (not (> (.chanceforcombocancel (Utilities|Array|Get(acopy) (Variables|Default|GetAttackMontageArray) (Variables|Default|GetCurrentComboIndex))) (Math|Random|RandomFloat)))
                    (goto _label)))))))))))

(event Custom|EndAbility
  (Ability|EndAbility))

(event Custom|BindHitboxActive
  (bind _returnvalue (Utilities|Time|SetTimerbyEvent (EventDispatchers|CreateEvent :!event RunHitboxTrace) 0.0001 true true))
  (Variables|Default|SetHitboxTraceTimerHandle _returnvalue)
  (bind (_asynctaskproxy _payload) (Ability|Tasks|WaitGameplayEvent "(TagName=\"Combat.Event.HitActor\")" 0)
    (:then
      (Variables|Default|SetWaitHitActorTask _asynctaskproxy))
    (:EventReceived
      (Utilities|IsValid (Ability|GetAbilitySystemComponent (.Target (Utilities|Struct|BreakGameplayEventData _payload)))
        (:Is%20Valid
          (CallFunction|HandleHit (Ability|TargetData|GetHitResultfromTargetData (.TargetData (Utilities|Struct|BreakGameplayEventData _payload)))))
        (:Is%20Not%20Valid
          (Variables|Default|SetComboInterrupted true)
          (Variables|Default|SetShouldCombo false)
          (CallFunction|HandleNonHit (Ability|TargetData|GetHitResultfromTargetData (.TargetData (Utilities|Struct|BreakGameplayEventData _payload)))))))))

(event Custom|UnbindHitboxActive
  (Utilities|Time|ClearandInvalidateTimerbyHandle (Variables|Default|GetHitboxTraceTimerHandle)))

(event Custom|HandleParry
  (params (Hit :type Hit%20Result%20Structure))
  (bind _hitactor (Collision|BreakHitResult Hit))
  (bind _returnvalue (Class|CombatInterface|GetOwnerWeapon(Message) _hitactor))
  (Abilities|TryActivateAbilitiesbyTag (Ability|GetAbilitySystemComponent _hitactor) (GameplayTags|MakeGameplayTagContainerfromTag "(TagName=\"Combat.Ability.BlockImpact\")") true)
  (bind _returnvalue_2 (Ability|GameplayEffect|AssignTagSetbyCallerMagnitude (Ability|MakeOutgoingGameplayEffectSpec "/Game/GAS/GameplayEffects/GE_AlterPosture.GE_AlterPosture_C") "(TagName=\"GameplayEffect.Posture\")" (Math|Conversions|ToFloat(Integer) (Math|Random|RandomIntegerinRange (Variables|/Script/GASAssignment.PDA_WeaponBaseData|GetLowerPostureDamageRange (Variables|/Script/GASAssignment.Weapon|GetWeaponBaseData _returnvalue)) (Variables|/Script/GASAssignment.PDA_WeaponBaseData|GetUpperPostureDamageRange (Variables|/Script/GASAssignment.Weapon|GetWeaponBaseData _returnvalue))))))
  (GameplayEffects|ApplyGameplayEffectSpecToSelf (Ability|GetAbilitySystemComponentfromActorInfo) _returnvalue_2)
  (GameplayCue|ExecuteGameplayCue :GameplayCueTag "(TagName=\"GameplayCue.Parry\")")
  (if (> (.chanceforcombointerruption (Utilities|Array|Get(acopy) (Variables|Default|GetAttackMontageArray) (Variables|Default|GetCurrentComboIndex))) (Math|Random|RandomFloat))
    (Variables|Default|SetComboInterrupted true)
    (CallFunction|StopCurrentMontage)
    (Abilities|TryActivateAbilitiesbyTag (Ability|GetAbilitySystemComponentfromActorInfo) (GameplayTags|MakeGameplayTagContainerfromTag "(TagName=\"Combat.Ability.NonHitImpact\")") true)
    (CallFunction|EndAbility)))

(event Custom|HandleBlock
  (params (Hit :type Hit%20Result%20Structure))
  (bind _hitactor (Collision|BreakHitResult Hit))
  (bind _returnvalue (Ability|GetAbilitySystemComponent _hitactor))
  (Abilities|TryActivateAbilitiesbyTag _returnvalue (GameplayTags|MakeGameplayTagContainerfromTag "(TagName=\"Combat.Ability.BlockImpact\")") true)
  (bind _returnvalue_2 (Ability|GameplayEffect|AssignTagSetbyCallerMagnitude (Ability|MakeOutgoingGameplayEffectSpec "/Game/GAS/GameplayEffects/GE_AlterPosture.GE_AlterPosture_C") "(TagName=\"GameplayEffect.Posture\")" 2.5))
  (GameplayEffects|ApplyGameplayEffectSpecToSelf _returnvalue _returnvalue_2)
  (GameplayCue|ExecuteGameplayCueOnActor(Burst) _hitactor "(TagName=\"GameplayCue.Block\")" (Ability|GameplayCue|MakeGameplayCueParameters 0.0)))

(event Custom|HandleHit
  (params (Hit :type Hit%20Result%20Structure))
  (bind (_bblockinghit _binitialoverlap _time _distance _location _impactpoint _normal _impactnormal _physmat _hitactor) (Collision|BreakHitResult Hit))
  (bind _ownerweapon (Variables|Default|GetOwnerWeapon))
  (bind _returnvalue (Ability|GetAbilitySystemComponent _hitactor))
  (bind _weaponbasedata (Variables|/Script/GASAssignment.Weapon|GetWeaponBaseData _ownerweapon))
  (if (< (Math|Vector|DotProduct (Variables|Default|GetOwnerForwardVector) (Transformation|GetActorForwardVector _hitactor)) -0.1)
    (if (GameplayTags|HasMatchingGameplayTag _returnvalue "(TagName=\"Combat.State.Parrying\")")
      (CallFunction|HandleParry Hit)
      (elif (GameplayTags|HasMatchingGameplayTag _returnvalue "(TagName=\"Combat.State.Blocking\")")
        (CallFunction|HandleBlock Hit)
        (else
          (bind _returnvalue_2 (Ability|GameplayEffect|AssignTagSetbyCallerMagnitude (Ability|MakeOutgoingGameplayEffectSpec "/Game/GAS/GameplayEffects/GE_AlterHealth.GE_AlterHealth_C") "(TagName=\"GameplayEffect.Health\")" (* (Math|Conversions|ToFloat(Integer) (Math|Random|RandomIntegerinRange (Variables|/Script/GASAssignment.PDA_WeaponBaseData|GetLowerHealthDamageRange _weaponbasedata) (Variables|/Script/GASAssignment.PDA_WeaponBaseData|GetUpperHealthDamageRange _weaponbasedata))) -1.0) :!label _label))
          (GameplayEffects|ApplyGameplayEffectSpecToSelf _returnvalue _returnvalue_2)
          (GameplayCue|ExecuteGameplayCueOnActor(Burst) _hitactor "(TagName=\"GameplayCue.Hit\")" (Ability|GameplayCue|MakeGameplayCueParameters :Location _location))
          (if (> (Math|Random|RandomFloat) 0.67)
            (Abilities|TryActivateAbilitiesbyTag _returnvalue (GameplayTags|MakeGameplayTagContainerfromTag "(TagName=\"Combat.Ability.HitImpact\")") true)))))
    (else
      (goto _label))))

(event Custom|HandleNonHit
  (params (Hit :type Hit%20Result%20Structure))
  (CallFunction|StopCurrentMontage)
  (Abilities|TryActivateAbilitiesbyTag (Ability|GetAbilitySystemComponentfromActorInfo) (GameplayTags|MakeGameplayTagContainerfromTag "(TagName=\"Combat.Ability.NonHitImpact\")") true)
  (Class|GameplayAbility|ExecuteGameplayCuewithParams "(TagName=\"GameplayCue.NonHit\")" (Ability|GameplayCue|MakeGameplayCueParameters :Location (.Location (Collision|BreakHitResult Hit))))
  (CallFunction|EndAbility))

(event Ability|EventOnEndAbility
  (params (bWasCancelled :type Boolean))
  (bind _waithitactortask (Variables|Default|GetWaitHitActorTask))
  (bind _ownerweapon (Variables|Default|GetOwnerWeapon))
  (Ability|GameplayEffect|RemoveLooseGameplayTags (Ability|GetOwningActorfromActorInfo) (GameplayTags|MakeLiteralGameplayTagContainer "(GameplayTags=((TagName=\"Combat.State.Attacking.HitboxActive\"),(TagName=\"Combat.State.Attacking.ComboActive\")))"))
  (Utilities|IsValid _waithitactortask
    (:Is%20Valid
      (GameplayTasks|EndTask _waithitactortask))
    (:Is%20Not%20Valid
      _))
  (Utilities|IsValid _ownerweapon
    (:Is%20Valid
      (Class|Weapon|ResetIgnoreArray _ownerweapon))
    (:Is%20Not%20Valid
      _))
  (CallFunction|ResettoDefault)
  (Development|PrintString "resetting"))

(event Ability|EventActivateAbility
  (bind _returnvalue (Ability|GetOwningActorfromActorInfo))
  (bind _returnvalue_2 (Ability|GetOwningActorfromActorInfo))
  (bind _waithitactortask (Variables|Default|GetWaitHitActorTask))
  (CallFunction|WaitforComboInput)
  (bind _returnvalue_3 (Class|CombatInterface|GetOwnerWeapon(Message) (Ability|GetOwningActorfromActorInfo)))
  (bind _output_get (Variables|Default|SetOwnerWeapon _returnvalue_3))
  (Utilities|IsValid _output_get
    (:Is%20Valid
      (Utilities|IsValid (Variables|/Script/GASAssignment.Weapon|GetWeaponAnimationData _output_get)
        (:Is%20Valid
          (Variables|Default|SetOwnerCMC (.AsCharacter%20Movement%20Component (Utilities|Casting|CastToCharacterMovementComponent (.MovementComponent (Utilities|Struct|BreakGameplayAbilityActorInfo (Ability|GetActorInfo))))))
          (Variables|Default|SetOwnerForwardVector (Transformation|GetActorForwardVector (Ability|GetOwningActorfromActorInfo)))
          (Variables|Default|SetIsAIControlled (Utilities|IsValid (AI|GetAIController (Utilities|Struct|BreakGameplayAbilityActorInfo (Ability|GetActorInfo)))))
          (bind _returnvalue_4 (Ability|CommitAbility))
          (if _returnvalue_4
            (CallFunction|ResolveMontagestoUse)
            (Variables|Default|SetShouldCombo false)
            (bind _notifyname (Animation|Montage|PlayMontage (Utilities|Struct|BreakGameplayAbilityActorInfo (Ability|GetActorInfo)) (.montage (Utilities|Array|Get(acopy) (Variables|Default|GetAttackMontageArray) (Variables|Default|GetCurrentComboIndex))))
              (:OnBlendOut
                (CallFunction|EndAbility))
              (:OnNotifyBegin
                (switch name _notifyname
                  (:HitboxActive
                    (Ability|GameplayEffect|AddLooseGameplayTags _returnvalue_2 (GameplayTags|MakeGameplayTagContainerfromTag "(TagName=\"Combat.State.Attacking.HitboxActive\")"))
                    (CallFunction|BindHitboxActive)
                    (Audio|PlaySoundatLocation "/Game/Sounds/SC_Slash.SC_Slash" (Transformation|GetActorLocation (Utilities|Struct|BreakGameplayAbilityActorInfo (Ability|GetActorInfo))) "0, 0, 0" 1.0 1.0 0.0 0 0 0 0))
                  (:ComboWindow
                    (Ability|GameplayEffect|AddLooseGameplayTags _returnvalue_2 (GameplayTags|MakeGameplayTagContainerfromTag "(TagName=\"Combat.State.Attacking.ComboActive\")")))))
              (:OnNotifyEnd
                (if (Class|AbilitySystemBlueprintLibrary|IsGameplayAbilityActive)
                  (switch name _notifyname
                    (:HitboxActive
                      (Ability|GameplayEffect|RemoveLooseGameplayTags _returnvalue (GameplayTags|MakeGameplayTagContainerfromTag "(TagName=\"Combat.State.Attacking.HitboxActive\")"))
                      (CallFunction|UnbindHitboxActive)
                      (Utilities|IsValid _waithitactortask
                        (:Is%20Valid
                          (GameplayTasks|EndTask _waithitactortask))
                        (:Is%20Not%20Valid
                          _))
                      (Utilities|IsValid (Variables|Default|GetOwnerWeapon)
                        (:Is%20Valid
                          (Class|Weapon|ResetIgnoreArray (Variables|Default|GetOwnerWeapon)))))
                    (:ComboWindow
                      (Ability|GameplayEffect|RemoveLooseGameplayTags _returnvalue (GameplayTags|MakeGameplayTagContainerfromTag "(TagName=\"Combat.State.Attacking.ComboActive\")"))
                      (if (Variables|Default|GetShouldCombo)
                        (bind _result (Math|Integer|IncrementInt (Variables|Default|GetCurrentComboIndex) :!label _label)
                          (:%20%20
                            (if (not (> _result (Utilities|Array|LastIndex (Variables|Default|GetAttackMontageArray))))
                              (CallFunction|TriggerNextCombo))))
                        (elif (Variables|Default|GetIsAIControlled)
                          (if (not (> (.chanceforcombocancel (Utilities|Array|Get(acopy) (Variables|Default|GetAttackMontageArray) (Variables|Default|GetCurrentComboIndex))) (Math|Random|RandomFloat)))
                            (goto _label)))))))))
            (else
              (CallFunction|EndAbility :!label _label_2))))
        (:Is%20Not%20Valid
          (goto _label_2))))
    (:Is%20Not%20Valid
      (goto _label_2))))

(fn RunHitboxTrace
  (bind _ownerweapon (Variables|Default|GetOwnerWeapon))
  (Utilities|IsValid _ownerweapon
    (:Is%20Valid
      (Class|Weapon|RunWeaponTrace _ownerweapon))))

(fn StopCurrentMontage
  (bind _returnvalue (Ability|GetActorInfo))
  (bind _skeletalmeshcomponent (Utilities|Struct|BreakGameplayAbilityActorInfo _returnvalue))
  (bind _returnvalue_2 (Components|SkeletalMesh|GetAnimInstance _skeletalmeshcomponent))
  (Animation|Montage|MontageStop _returnvalue_2 0.1 (Animation|Montage|GetCurrentActiveMontage _returnvalue_2)))

(fn ResettoDefault
  (bind (_ownerweapon _currentcomboindex _shouldcombo _combointerrupted _hitboxtracetimerhandle _candamage) (Utilities|GetClassDefaults "GA_Attack_C"))
  (Variables|Default|SetOwnerWeapon _ownerweapon)
  (Variables|Default|SetCurrentComboIndex _currentcomboindex)
  (Variables|Default|SetComboInterrupted _combointerrupted)
  (Variables|Default|SetShouldCombo _shouldcombo)
  (Variables|Default|SetCanDamage _candamage)
  (Utilities|Time|ClearandInvalidateTimerbyHandle (Variables|Default|GetHitboxTraceTimerHandle)))

(fn ResolveMontagestoUse
  (Variables|Default|SetAttackMontageArray (Variables|/Script/GASAssignment.PDA_WeaponAnimationData|GetComboData (Variables|/Script/GASAssignment.Weapon|GetWeaponAnimationData (Variables|Default|GetOwnerWeapon)))))