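; Gameplay ability for blocking and parrying that plays the owner weapon's block montage and ends when it blends out.
; Montage notify windows add and remove loose Parrying and Blocking tags, with a flag allowing only one parry window per activation.
; Releasing input or gaining the Block.End tag jumps the montage to its Exit section.
; Ending the ability clears the Blocking tag and resets the parry flag.
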(event Custom|WaitForEndBlock
  (Ability|Tasks|WaitInputRelease false
    (:then
      (Ability|Tasks|WaitGameplayTagAdd "(TagName=\"Combat.Ability.Block.End\")" 0 true
        (:Added
          _)))
    (:OnRelease
      _))
  (Ability|Animation|MontageJumptoSection (Components|SkeletalMesh|GetAnimInstance (Utilities|Struct|BreakGameplayAbilityActorInfo (Ability|GetActorInfo))) "Exit" (Variables|/Script/GASAssignment.PDA_WeaponAnimationData|GetBlockMontage (Variables|/Script/GASAssignment.Weapon|GetWeaponAnimationData (Variables|Default|GetOwnerWeapon)))))

(event Ability|EventOnEndAbility
  (params (bWasCancelled :type Boolean))
  (Ability|GameplayEffect|RemoveLooseGameplayTags (Ability|GetOwningActorfromActorInfo) (GameplayTags|MakeGameplayTagContainerfromTag "(TagName=\"Combat.State.Blocking\")"))
  (Variables|Default|SetHasParryEnded false))

(event Ability|EventActivateAbility
  (bind _returnvalue (Ability|GetOwningActorfromActorInfo))
  (bind _returnvalue_2 (GameplayTags|MakeGameplayTagContainerfromTag "(TagName=\"Combat.State.Parrying\")"))
  (bind _returnvalue_3 (Ability|GetOwningActorfromActorInfo))
  (bind _returnvalue_4 (GameplayTags|MakeGameplayTagContainerfromTag "(TagName=\"Combat.State.Blocking\")"))
  (CallFunction|WaitforEndBlock)
  (bind _returnvalue_5 (Class|CombatInterface|GetOwnerWeapon(Message) (Ability|GetOwningActorfromActorInfo)))
  (bind _output_get (Variables|Default|SetOwnerWeapon _returnvalue_5))
  (Utilities|IsValid _output_get
    (:Is%20Valid
      (Utilities|IsValid (Variables|/Script/GASAssignment.Weapon|GetWeaponAnimationData _output_get)
        (:Is%20Valid
          (bind _returnvalue_6 (Ability|CommitAbility))
          (if _returnvalue_6
            (bind _notifyname (Animation|Montage|PlayMontage (Utilities|Struct|BreakGameplayAbilityActorInfo (Ability|GetActorInfo)) (Variables|/Script/GASAssignment.PDA_WeaponAnimationData|GetBlockMontage (Variables|/Script/GASAssignment.Weapon|GetWeaponAnimationData (Variables|Default|GetOwnerWeapon))))
              (:OnBlendOut
                (Ability|EndAbility))
              (:OnNotifyBegin
                (switch name _notifyname
                  (:ParryActive
                    (if (not (Variables|Default|GetHasParryEnded))
                      (Ability|GameplayEffect|AddLooseGameplayTags _returnvalue _returnvalue_2)))
                  (:BlockActive
                    (Ability|GameplayEffect|AddLooseGameplayTags _returnvalue _returnvalue_4))))
              (:OnNotifyEnd
                (switch name _notifyname
                  (:ParryActive
                    (Ability|GameplayEffect|RemoveLooseGameplayTags _returnvalue_3 _returnvalue_2)
                    (Variables|Default|SetHasParryEnded true))
                  (:BlockActive
                    (Ability|GameplayEffect|RemoveLooseGameplayTags _returnvalue_3 _returnvalue_4)))))
            (else
              (Ability|EndAbility :!label _label))))
        (:Is%20Not%20Valid
          (goto _label))))
    (:Is%20Not%20Valid
      (goto _label))))