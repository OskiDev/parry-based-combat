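; Gameplay ability that sheathes the owner's current weapon and returns it to its default socket on the character's mesh.
; It gets the weapon from the owning actor, validates its base and animation data, and commits, ending immediately if any check fails.
; It plays the weapon's slowed sheathe montage, then on blend out resets the transform, reattaches the weapon, applies GE_WeaponUnequipped and ends.
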(event Ability|EventActivateAbility
  (bind _returnvalue (Class|CombatInterface|GetOwnerWeapon(Message) (Utilities|Struct|BreakGameplayAbilityActorInfo (Ability|GetActorInfo))))
  (bind _output_get (Variables|Default|SetOwnerWeapon%20 _returnvalue))
  (Utilities|IsValid _output_get
    (:Is%20Valid
      (Utilities|IsValid (Variables|/Script/GASAssignment.Weapon|GetWeaponBaseData _output_get)
        (:Is%20Valid
          (Utilities|IsValid (Variables|/Script/GASAssignment.Weapon|GetWeaponAnimationData _output_get)
            (:Is%20Valid
              (bind _returnvalue_2 (Ability|CommitAbility))
              (if _returnvalue_2
                (|PlayMontageandWaitProxy "None" (Variables|/Script/GASAssignment.PDA_WeaponAnimationData|GetSheatheWeaponMontage (Variables|/Script/GASAssignment.Weapon|GetWeaponAnimationData (Variables|Default|GetOwnerWeapon%20))) 0.75 "None" false 1.0 0.0 false
                  (:OnBlendOut
                    (Transformation|SetActorRelativeTransform (Variables|Default|GetOwnerWeapon%20) (Variables|/Script/GASAssignment.PDA_WeaponBaseData|GetDefaultWeaponTransform (Variables|/Script/GASAssignment.Weapon|GetWeaponBaseData (Variables|Default|GetOwnerWeapon%20))) false false)
                    (Transformation|AttachComponentToComponent (Variables|Default|GetOwnerWeapon%20) (Utilities|Struct|BreakGameplayAbilityActorInfo (Ability|GetActorInfo)) (Variables|/Script/GASAssignment.PDA_WeaponBaseData|GetDefaultSocket (Variables|/Script/GASAssignment.Weapon|GetWeaponBaseData (Variables|Default|GetOwnerWeapon%20))) "KeepRelative" "KeepRelative" "KeepRelative" false)
                    (Ability|ApplyGameplayEffectToOwner "/Game/GAS/GameplayEffects/GE_WeaponUnequipped.GE_WeaponUnequipped_C")
                    (Ability|EndAbility)))
                (else
                  (Ability|EndAbility :!label _label))))
            (:Is%20Not%20Valid
              (goto _label))))
        (:Is%20Not%20Valid
          (goto _label))))
    (:Is%20Not%20Valid
      (goto _label))))