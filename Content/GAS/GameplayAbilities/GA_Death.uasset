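; GA_Death is a Gameplay Ability that handles death for GAS base characters, turning a death animation into a ragdoll.
; Both direct and event-triggered activation commit the ability, then play AM_Death on the actor info's skeletal mesh.
; A montage notify or an interruption calls DeathRagdoll on the owning GASBaseCharacter and ends the ability.
; Normal montage completion has no handler, so the handoff relies on those two callbacks.
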(event Ability|EventActivateAbility
  (bind _returnvalue (Ability|CommitAbility))
  (if _returnvalue
    (bind _notifyname (Animation|Montage|PlayMontage (Utilities|Struct|BreakGameplayAbilityActorInfo (Ability|GetActorInfo)) "/Game/Characters/AlienSoldier/Animations/Sword/Death/AM_Death.AM_Death")
      (:OnInterrupted
        _)
      (:OnNotifyBegin
        (switch name _notifyname
          (:Ragdoll
            _))))
    (bind _asgasbase_character (Utilities|Casting|CastToGASBaseCharacter (Utilities|Struct|BreakGameplayAbilityActorInfo (Ability|GetActorInfo))))
    (Class|GASBaseCharacter|DeathRagdoll _asgasbase_character)
    (Ability|EndAbility)))

(event Ability|EventActivateAbilityFromEvent
  (params (EventData :type Gameplay%20Event%20Data%20Structure%20%28by%20ref%29))
  (bind _returnvalue (Ability|CommitAbility))
  (if _returnvalue
    (bind _notifyname (Animation|Montage|PlayMontage (Utilities|Struct|BreakGameplayAbilityActorInfo (Ability|GetActorInfo)) "/Game/Characters/AlienSoldier/Animations/Sword/Death/AM_Death.AM_Death")
      (:OnInterrupted
        _)
      (:OnNotifyBegin
        (switch name _notifyname
          (:Ragdoll
            _))))
    (bind _asgasbase_character (Utilities|Casting|CastToGASBaseCharacter (Utilities|Struct|BreakGameplayAbilityActorInfo (Ability|GetActorInfo))))
    (Class|GASBaseCharacter|DeathRagdoll _asgasbase_character)
    (Ability|EndAbility)))