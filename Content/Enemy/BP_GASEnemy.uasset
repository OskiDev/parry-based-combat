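; BP_GASEnemy is an enemy character that uses Gameplay Ability System tags to react to its death.
; On BeginPlay it waits for the Combat.State.IsDead tag; when that tag is added it destroys its widget component and stops the brain logic on its AIC_Enemy controller.
; A disconnected node chain that would turn it toward the player character is never run.
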(event EventBeginPlay
  (Ability|Tasks|WaitGameplayTagAddToActor 0 "(TagName=\"Combat.State.IsDead\")"
    (:Added
      (Components|DestroyComponent (Variables|Default|GetWidget))
      (bind _asaic_enemy (Utilities|Casting|CastToAIC_Enemy (Pawn|GetController)))
      (AI|Logic|StopLogic (Variables|/Script/AIModule.AIController|GetBrainComponent _asaic_enemy) ""))))

(event EventTick
  (params (DeltaSeconds :type Float%20%28single-precision%29)))

(fn ConstructionScript)