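; Sword weapon actor that detects melee hits and reports them to its owner through the Gameplay Ability System.
; RunWeaponTrace sphere-sweeps the Visibility channel between the mesh's TraceStart and TraceEnd sockets, with debug drawing.
; Each hit actor is sent to the owner as a Combat.Event.HitActor event with hit-result target data.
; Hit actors join an ignore array, reset on BeginPlay, so later traces skip them.
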(event EventBeginPlay
  (Class|Weapon|ResetIgnoreArray))

(fn ConstructionScript)

(fn RunWeaponTrace
  (bind _returnvalue (Components|GetOwner))
  (bind _staticmeshcomp (Variables|Default|GetStaticMeshComp))
  (bind _outhits (Collision|MultiSphereTraceByChannel (Transformation|GetSocketLocation _staticmeshcomp "TraceStart") (Transformation|GetSocketLocation _staticmeshcomp "TraceEnd") 15.0 "TraceTypeQuery1" false (Variables|Default|GetTraceIgnoreArray) "ForOneFrame"))
  (for _array_element _outhits
    (Utilities|IsValid (.HitActor (Collision|BreakHitResult _array_element))
      (:Is%20Valid
        (Ability|SendGameplayEventtoActor _returnvalue "(TagName=\"Combat.Event.HitActor\")" (Utilities|Struct|MakeGameplayEventData _returnvalue (.HitActor (Collision|BreakHitResult _array_element)) (Ability|TargetData|AbilityTargetDatafromHitResult _array_element)))
        (Utilities|Array|AddUnique (Variables|Default|GetTraceIgnoreArray) (.HitActor (Collision|BreakHitResult _array_element))))))
  (return))